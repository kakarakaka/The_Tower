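; Enemy character AI Blueprint that chases the player and plays an attack montage on arrival.
; PawnSensing sightings set a seen flag and call FollowPlayer, which runs AI MoveTo and gates attacks with a flag and montage-length delay.
; StunEnemy halts movement and blocks attacks for a timed duration, while RecoverFromStun resumes the chase if the seen flag is set.
; Tick stops movement whenever that flag is false.
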(event `self.ReceiveTick`
  (params (DeltaSeconds :type "Float (single-precision)"))
  (if (not (`self.IsSeeingPlayer`))
    (`MovementComponent.StopMovementImmediately` (`self.CharacterMovement`))))

(event `self.PawnSensing.OnSeePawn`
  (params (Pawn :type "Pawn Object Reference"))
  (set `self.IsSeeingPlayer` true)
  (`self.FollowPlayer`))

(event `FollowPlayer`
  (if (not (`self.IsStunned`))
    (set `self.CanAtack` true)
    (if (`self.IsSeeingPlayer`)
      (`|AIMoveTo` self (0.0 0.0 0.0) (`GameplayStatics.GetPlayerCharacter` 0) 50.0
        (:`OnSuccess`
          (if (`self.CanAtack`)
            (set `self.CanAtack` false)
            (bind _returnvalue (`self.PlayAnimMontage` null))
            (`KismetSystemLibrary.Delay` _returnvalue)
            (set `self.CanAtack` true))))
      (else
        (set `self.IsSeeingPlayer` false)))))

(event `StunEnemy`
  (set `self.IsStunned` true)
  (set `self.CanAtack` false)
  (bind _asaicontroller (cast `AIController` (`self.GetController`)))
  (`Controller.StopMovement` _asaicontroller)
  (`MovementComponent.StopMovementImmediately` (`self.CharacterMovement`))
  (`KismetSystemLibrary.K2_SetTimerDelegate` (`|CreateDelegate` :!event `RecoverFromStun`) (`self.StunDuration`)))

(event `RecoverFromStun`
  (set `self.IsStunned` false)
  (if (`self.IsSeeingPlayer`)
    (`self.FollowPlayer`)
    (else
      (set `self.CanAtack` true))))

(fn `UserConstructionScript`)